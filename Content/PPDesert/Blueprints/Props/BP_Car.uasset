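; BP_Car is a car prop that randomizes its mesh variation and paint when its GenerateCar event runs.
; RandomGenerator picks the hatchback, pickup or wagon mesh array from CarType, then sets a random mesh from it.
; A dynamic material instance, built from the array's first mesh, receives either a random palette color and leaf multiplier or the specified paint color, depending on RandomColor.
; The construction script and BeginPlay are empty, so neither triggers generation.
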(event `GenerateCar`
  (`self.RandomGenerator`))

(fn `RandomGenerator`
  (bind _activearray (`self.ActiveArray`))
  (bind _carbodymatinst (`self.CarBodyMatInst`))
  (bind _carcolors (`self.CarColors`))
  ;[1 1 1] Set Vehicle Type
  (bind _output_get (set `self.ActiveArray` (select `byte` (`self.CarType`) :`0` (`self.CarVariationsHatchback`) :`1` (`self.CarVariationsPickup`) :`2` (`self.CarVariationsWagon`))))
  ;[1 1 1] Create Material Instance
  (bind _returnvalue (`PrimitiveComponent.CreateDynamicMaterialInstance` (`self.Car`) 0 (`StaticMesh.GetMaterial` (`|GetArrayItem` _output_get) 0) "None"))
  (set `self.CarBodyMatInst` _returnvalue)
  ;[1 1 1] Set Mesh Variation
  (bind _output_get_2 (set `self.MeshIndex` (`KismetMathLibrary.RandomInteger` (`KismetArrayLibrary.Array_Length` _activearray))))
  (`StaticMeshComponent.SetStaticMesh` (`self.Car`) (`|GetArrayItem` _activearray _output_get_2))
  (if (`self.RandomColor`)
    ;[1 1 1] Generate Random Color
    (`MaterialInstanceDynamic.SetVectorParameterValue` _carbodymatinst "AlbedoColor" (`|GetArrayItem` _carcolors (`KismetMathLibrary.RandomInteger` (`KismetArrayLibrary.Array_Length` _carcolors))))
    (`MaterialInstanceDynamic.SetScalarParameterValue` _carbodymatinst "LeafsMultiplier" (`KismetMathLibrary.RandomFloatInRange` 2.0 6.0))
    (else
      ;[1 1 1] Generate Color
      (`MaterialInstanceDynamic.SetVectorParameterValue` (`self.CarBodyMatInst`) "AlbedoColor" (`self.CarPaintColor`)))))

(fn `UserConstructionScript`)