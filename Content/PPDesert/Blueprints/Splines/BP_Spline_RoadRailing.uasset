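; Spline-driven road railing that builds a line of railing meshes along its spline in the construction script.
; It divides the spline length by Spacing and adds a manually attached, collision-enabled spline mesh per interval, using world-space positions and directions scaled by TangentScale.
; Generation runs only when DisableForFasterEditing is true, despite the flag's name.
; The event graph has no runtime logic.
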(fn `UserConstructionScript`
  (bind _spline (`self.Spline`))
  (bind _spacing (`self.Spacing`))
  (bind _tangentscale (`self.TangentScale`))
  (if (`self.DisableForFasterEditing`)
    (for _index (range (+ (`.ReturnValue` (`KismetMathLibrary.FMod` (`SplineComponent.GetSplineLength` _spline) _spacing)) 1))
      (bind _returnvalue (`AddComponent|NODE_AddSplineMeshComponent-5` :`bManualAttachment` true))
      (`PrimitiveComponent.SetCollisionEnabled` _returnvalue "QueryAndPhysics")
      (`StaticMeshComponent.SetStaticMesh` _returnvalue "/Game/PPDesert/Assets/Models/Items/Props/SM_OutsideRoadRailingLine.SM_OutsideRoadRailingLine")
      (bind _returnvalue_2 (* _index _spacing))
      (bind _returnvalue_3 (+ _returnvalue_2 _spacing))
      (`SplineMeshComponent.SetStartAndEnd` _returnvalue (`SplineComponent.GetLocationAtDistanceAlongSpline` _spline _returnvalue_2 "World") (* (`SplineComponent.GetDirectionAtDistanceAlongSpline` _spline _returnvalue_2 "World") _tangentscale) (`SplineComponent.GetLocationAtDistanceAlongSpline` _spline _returnvalue_3 "World") (* (`SplineComponent.GetDirectionAtDistanceAlongSpline` _spline _returnvalue_3 "World") _tangentscale) true))))